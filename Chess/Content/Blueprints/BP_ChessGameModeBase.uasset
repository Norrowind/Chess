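; BP_ChessGameModeBase is the chess game mode Blueprint that handles the end-of-game win or lose screen.
; ShowWinorLoose creates either the WBP_PlayerWin or WBP_PlayerLoose widget from a PlayerWin flag, stores it in ScreenMessage and adds it to the viewport.
; HideWinorLoose removes that stored widget from its parent if it is still valid.
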(event EventShowWinorLoose
  (params (bPlayerWin :type Boolean))
  (if bPlayerWin
    (bind _returnvalue (UserInterface|CreateWidget "/Game/UI/WBP_PlayerWin.WBP_PlayerWin_C"))
    (Variables|Default|SetScreenMessage _returnvalue)
    (UserInterface|Viewport|AddtoViewport _returnvalue 0)
    (else
      (bind _returnvalue_2 (UserInterface|CreateWidget "/Game/UI/WBP_PlayerLoose.WBP_PlayerLoose_C"))
      (Variables|Default|SetScreenMessage _returnvalue_2)
      (UserInterface|Viewport|AddtoViewport _returnvalue_2 0))))

(event EventHideWinorLoose
  (bind _screenmessage (Variables|Default|GetScreenMessage))
  (Utilities|IsValid _screenmessage
    (:Is%20Valid
      (Widget|RemovefromParent _screenmessage))))

(fn ConstructionScript)